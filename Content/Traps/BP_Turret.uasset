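; Turret trap that fires BP_Projectile actors from its Scene component's location and rotation.
; A one-shot timer set at BeginPlay calls CallShoot after a short delay, starting a looping timer that drives Shoot.
; CallShoot uses a FlipFlop to alternate between starting and pausing fire, but nothing in this graph calls it again, so firing continues once started.
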(event Custom|Shoot
  (bind _scene (Variables|Default|GetScene))
  (bind _returnvalue (Transformation|GetWorldTransform _scene))
  (Game|SpawnActorfromClass "/Game/Traps/BP_Projectile.BP_Projectile_C" (Math|Transform|MakeTransform (.location _returnvalue) (.rotation _returnvalue) "1.000000,1.000000,1.000000") "Undefined" "MultiplyWithRoot" 0 0))

(event Custom|CallShoot
  (Utilities|FlowControl|FlipFlop
    (:A
      (bind _returnvalue (Utilities|Time|SetTimerbyEvent (delegate Custom|Shoot) 1.0 true false -1.0))
      (Variables|Default|SetShootTimer _returnvalue))
    (:B
      (Utilities|Time|PauseTimerbyHandle (Variables|Default|GetShootTimer)))))

(event EventBeginPlay
  (Utilities|Time|SetTimerbyEvent (delegate Custom|CallShoot) 5.0))

(event Collision|EventActorBeginOverlap
  (params (OtherActor :type Actor%20Object%20Reference)))

(event EventTick
  (params (DeltaSeconds :type Float%20%28single-precision%29)))

(fn ConstructionScript)