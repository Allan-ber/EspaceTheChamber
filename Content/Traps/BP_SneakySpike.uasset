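; BP_SneakySpike is a trap that springs a cone spike up when the top-down player character steps into its trigger.
; Overlapping Box1 raises the Cone and the Box damage volume, and Box calls Dégats on any BP_TopDownCharacter it overlaps.
; After a short delay the Cone drops back, but Box1 is lowered instead of Box, so both volumes drift with each trigger.
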(event OnComponentBeginOverlap(Box)
  (params (OverlappedComponent :type Primitive%20Component%20Object%20Reference) (OtherActor :type Actor%20Object%20Reference) (OtherComp :type Primitive%20Component%20Object%20Reference) (OtherBodyIndex :type Integer) (bFromSweep :type Boolean) (SweepResult :type Hit%20Result%20Structure%20%28by%20ref%29))
  (bind _asbp_top_down_character (Utilities|Casting|CastToBP_TopDownCharacter OtherActor))
  (Default|Dégats _asbp_top_down_character))

(event OnComponentBeginOverlap(Box1)
  (params (OverlappedComponent :type Primitive%20Component%20Object%20Reference) (OtherActor :type Actor%20Object%20Reference) (OtherComp :type Primitive%20Component%20Object%20Reference) (OtherBodyIndex :type Integer) (bFromSweep :type Boolean) (SweepResult :type Hit%20Result%20Structure%20%28by%20ref%29))
  (bind _cone (Variables|Default|GetCone))
  (bind _box (Variables|Default|GetBox))
  (bind _box1 (Variables|Default|GetBox1))
  (bind _cone_2 (Variables|Default|GetCone))
  (Utilities|Casting|CastToBP_TopDownCharacter OtherActor)
  (Transformation|SetRelativeLocation _cone (Math|Vector|MakeVector 0.0 0.0 (+ (.z (Variables|/Script/Engine.SceneComponent|GetRelativeLocation _cone)) 1e+02)) false false)
  (Transformation|SetRelativeLocation _box (Math|Vector|MakeVector 0.0 0.0 (+ (.z (Variables|/Script/Engine.SceneComponent|GetRelativeLocation _box)) 1e+02)) false false)
  (Utilities|FlowControl|Delay 2.0)
  (Transformation|SetRelativeLocation _cone_2 (Math|Vector|MakeVector 0.0 0.0 (- (.z (Variables|/Script/Engine.SceneComponent|GetRelativeLocation _cone_2)) 1e+02)) false false)
  (Transformation|SetRelativeLocation _box1 (Math|Vector|MakeVector 0.0 0.0 (- (.z (Variables|/Script/Engine.SceneComponent|GetRelativeLocation _box1)) 1e+02)) false false))

(event Collision|EventActorBeginOverlap
  (params (OtherActor :type Actor%20Object%20Reference)))

(event EventTick
  (params (DeltaSeconds :type Float%20%28single-precision%29)))

(fn ConstructionScript)